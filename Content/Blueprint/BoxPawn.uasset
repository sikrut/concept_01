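; BoxPawn is a pawn that can be highlighted and selected with the mouse.
; Cursor events on its Box component drive an integer SelectionState: unselected, hovered or selected.
; Hovering shows a blue spotlight, and clicking swaps it for a red one.
; Cursor exit only clears the hover state, and the graph has no deselect path or handling of inputs to the selected pawn.
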(event OnClicked(Box)
  (params (TouchedComponent :type Primitive%20Component%20Object%20Reference) (ButtonPressed :type Key%20Structure))
  ;[0.1238 0.5573 0.6094] Setting a variable to track selection and toggling highlighting visibility.
  ; State Defs:
  ; state 0 - unselected and mouse not over object. cannot select.
  ; state 1 - unselected but mouse is over object. can select.
  ; state 2 - selected object and can be given inputs
  (Rendering|SetVisibility (Variables|Default|GetSpotLightBLUE) false false)
  (Rendering|SetVisibility (Variables|Default|GetSpotLightRED) true false)
  (Variables|Components|SetselectionState 2))

(event OnBeginCursorOver(Box)
  (params (TouchedComponent :type Primitive%20Component%20Object%20Reference))
  ;[0.1238 0.5573 0.6094] Setting a variable to track selection and toggling highlighting visibility.
  ; State Defs:
  ; state 0 - unselected and mouse not over object. cannot select.
  ; state 1 - unselected but mouse is over object. can select.
  ; state 2 - selected object and can be given inputs
  (if (== (Variables|Components|GetselectionState) 0)
    (Rendering|SetVisibility (Variables|Default|GetSpotLightBLUE) true false)
    (Variables|Components|SetselectionState 1)))

(event OnEndCursorOver(Box)
  (params (TouchedComponent :type Primitive%20Component%20Object%20Reference))
  ;[0.1238 0.5573 0.6094] Setting a variable to track selection and toggling highlighting visibility.
  ; State Defs:
  ; state 0 - unselected and mouse not over object. cannot select.
  ; state 1 - unselected but mouse is over object. can select.
  ; state 2 - selected object and can be given inputs
  (if (== (Variables|Components|GetselectionState) 1)
    (Rendering|SetVisibility (Variables|Default|GetSpotLightBLUE) false false)
    (Variables|Components|SetselectionState 0)))

(fn ConstructionScript)