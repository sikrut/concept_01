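; Character camera Blueprint that moves along fixed world X and Y axes from the MoveForward and MoveRight input axes.
; Each tick with none of W, A, S or D held, it applies movement input against the current velocity to decelerate, then zeroes velocity at or below a speed threshold.
; Tick also prints the current speed, and the control-rotation yaw node is left unused.
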(event EventTick
  (params (DeltaSeconds :type Float%20%28single-precision%29))
  (bind _returnvalue (Transformation|GetVelocity))
  (bind _returnvalue_2 (Game|GetPlayerController 0))
  (bind _returnvalue_3 (Math|Vector|VectorLength _returnvalue))
  ;[0.3659 0.8492 1] Decellerate camera speed and set = 0 if velocity below threshold (event tick)
  (Development|PrintString (Utilities|String|ToString(Float) _returnvalue_3))
  (if (not (Math|Boolean|ORBoolean (Game|Player|IsInputKeyDown _returnvalue_2 "W") (Game|Player|IsInputKeyDown _returnvalue_2 "A") (Game|Player|IsInputKeyDown _returnvalue_2 "S") (Game|Player|IsInputKeyDown _returnvalue_2 "D")))
    (if (<= _returnvalue_3 3e+02)
      (Variables|/Script/Engine.MovementComponent|SetVelocity (Pawn|GetMovementComponent) "0, 0, 0")
      (else
        (Pawn|Input|AddMovementInput (Transformation|GetVelocity) -1.0 false)))))

(event Input|AxisEvents|InputAxisMoveForward
  (params (AxisValue :type Float%20%28single-precision%29))
  ;[0.3659 0.8492 1] Camera Movement based on default inputs
  (Pawn|Input|AddMovementInput (Math|Vector|GetForwardVector "0, 0, 0") AxisValue false))

(event Input|AxisEvents|InputAxisMoveRight
  (params (AxisValue :type Float%20%28single-precision%29))
  ;[0.3659 0.8492 1] Camera Movement based on default inputs
  (Pawn|Input|AddMovementInput (Math|Vector|GetRightVector "0, 0, 0") AxisValue false))

(fn ConstructionScript)